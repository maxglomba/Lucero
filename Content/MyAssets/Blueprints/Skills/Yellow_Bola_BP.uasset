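; Yellow ball skill projectile that flies in a straight line for a limited lifetime.
; Tick counts down LifeTimer while moving the actor along its forward vector, scaled by Speed, without sweeping, then destroys it once the timer drops below zero.
; It has no hit or damage logic in its graphs, and a rotation reset based on the Lucero character's LookUp state is left unconnected.
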(event EventBeginPlay)

(event Collision|EventActorBeginOverlap
  (params (OtherActor :type Actor%20Object%20Reference)))

(event EventTick
  (params (DeltaSeconds :type Float%20%28single-precision%29))
  (if (>= (Variables|Default|GetlifeTimer) 0.0)
    (Variables|Default|SetlifeTimer (- (Variables|Default|GetlifeTimer) DeltaSeconds))
    (Transformation|SetActorLocation (+ (Transformation|GetActorLocation) (* (* (* (Math|Vector|GetForwardVector (Transformation|GetActorRotation)) 3e+02) (Variables|Default|GetSpeed)) DeltaSeconds)) false false)
    (else
      (Utilities|FlowControl|DoOnce false
        (:Completed
          (Actor|DestroyActor))))))

(fn ConstructionScript)