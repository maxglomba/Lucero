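; EnemySpell_BP is an enemy spell projectile that damages the player and can power up crystals.
; Tick moves it forward without sweep, scaled by Speed, and destroys it once LifeTimer runs out.
; Overlapping the player's CollisionCylinder reduces HP, spawns an explosion and destroys the spell, while touching an inactive Crystal_BP's TouchCollision activates its power and destroys it.
; The construction script falls back to DefaultDamage when Damage is zero.
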(event OnComponentBeginOverlap(skillCollision)
  (params (OverlappedComponent :type Primitive%20Component%20Object%20Reference) (OtherActor :type Actor%20Object%20Reference) (OtherComp :type Primitive%20Component%20Object%20Reference) (OtherBodyIndex :type Integer) (bFromSweep :type Boolean) (SweepResult :type Hit%20Result%20Structure%20%28by%20ref%29))
  (Utilities|FlowControl|Sequence
    (:then_0
      (if (and (Actor|ActorHasTag OtherActor "Player") (Utilities|Enum|Equal(Enum) (Utilities|GetObjectName OtherComp) "CollisionCylinder"))
        (bind _aslucero_character_bp (Utilities|Casting|CastToLuceroCharacter_BP OtherActor))
        (Default|ReduceHP _aslucero_character_bp (Variables|Default|Getdamage))
        (Effects|SpawnEmitteratLocation "/Game/StarterContent/Particles/P_Explosion.P_Explosion" (Transformation|GetActorLocation))
        (Actor|DestroyActor)))
    (:then_1
      (bind _ascrystal_bp (Utilities|Casting|CastToCrystal_BP OtherActor))
      (if (Utilities|Enum|Equal(Enum) (Utilities|GetObjectName OtherComp) "TouchCollision")
        (if (not (Variables|/Game/MyAssets/Blueprints/Collectables/Crystal_BP.Crystal_BP_C|GetisActivatedPower? _ascrystal_bp))
          (Default|ActivatePower _ascrystal_bp "NewEnumerator0" 1)
          (Actor|DestroyActor))))))

(event Collision|EventActorBeginOverlap
  (params (OtherActor :type Actor%20Object%20Reference)))

(event EventTick
  (params (DeltaSeconds :type Float%20%28single-precision%29))
  (if (>= (Variables|Default|GetlifeTimer) 0.0)
    (Variables|Default|SetlifeTimer (- (Variables|Default|GetlifeTimer) DeltaSeconds))
    (Transformation|SetActorLocation (+ (Transformation|GetActorLocation) (* (* (* (Math|Vector|GetForwardVector (Transformation|GetActorRotation)) 3e+02) (Variables|Default|GetSpeed)) DeltaSeconds)) false false)
    (else
      (Utilities|FlowControl|DoOnce false
        (:Completed
          (Actor|DestroyActor))))))

(fn ConstructionScript
  (if (== (Variables|Default|Getdamage) 0.0)
    (Variables|Default|Setdamage (Variables|Default|GetdefaultDamage))))