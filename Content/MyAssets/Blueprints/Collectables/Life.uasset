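; Life is a collectable health pickup that restores HP to the Lucero player character.
; On BeginPlay it spawns and plays a looping magic sound attached to its MediaSound component.
; When the character overlaps its sphere with HP below maximum, it adds HPRestore, stops the sound and destroys itself.
; At full health the pickup stays in place.
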(event OnComponentBeginOverlap(Sphere)
  (params (OverlappedComponent :type Primitive%20Component%20Object%20Reference) (OtherActor :type Actor%20Object%20Reference) (OtherComp :type Primitive%20Component%20Object%20Reference) (OtherBodyIndex :type Integer) (bFromSweep :type Boolean) (SweepResult :type Hit%20Result%20Structure%20%28by%20ref%29))
  (bind _aslucero_character_bp (Utilities|Casting|CastToLuceroCharacter_BP OtherActor))
  (if (< (Variables|/Game/MyAssets/Blueprints/Character/LuceroCharacter_BP.LuceroCharacter_BP_C|GetHP _aslucero_character_bp) (Variables|/Game/MyAssets/Blueprints/Character/LuceroCharacter_BP.LuceroCharacter_BP_C|GetHP_Max _aslucero_character_bp))
    (Default|AddHP _aslucero_character_bp (Variables|Default|GetHPRestore))
    (Audio|Components|Audio|StopDelayed (Variables|Default|GetmagicSound) 0.0)
    (Actor|DestroyActor)))

(event EventBeginPlay
  (bind _returnvalue (Audio|SpawnSoundAttached "/Game/MyAssets/Sounds/Loops/magic4_loop.magic4_loop" (Variables|Default|GetMediaSound) "None" "0, 0, 0" "0, 0, 0" "KeepRelativeOffset" false 1.0 1.0 0.0 "/Game/MyAssets/Sounds/Loops/config_attenuation_default.config_attenuation_default" 0))
  (bind _output_get (Variables|Default|SetmagicSound _returnvalue))
  (Audio|Components|Audio|Play _output_get 0.0))

(event Collision|EventActorBeginOverlap
  (params (OtherActor :type Actor%20Object%20Reference)))

(event EventTick
  (params (DeltaSeconds :type Float%20%28single-precision%29)))

(fn ConstructionScript)