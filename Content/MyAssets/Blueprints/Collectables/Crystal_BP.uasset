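; Collectable crystal that, while powered Yellow, Blue or Red, purifies, alters or slows nearby Pompon enemies by enemy type and color.
; ActivatePower sets material, light, particles and a timer from skill points; an aura-active player's touch triggers Red.
; Tick drains the timer, at a potentiated rate while being collected, and expiry unpurifies affected enemies.
; Collection adds a crystal to LuceroCharacter and destroys the actor, immediately if unpowered, otherwise once drained.
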(event OnComponentEndOverlap(TouchCollision)
  (params (OverlappedComponent :type Primitive%20Component%20Object%20Reference) (OtherActor :type Actor%20Object%20Reference) (OtherComp :type Primitive%20Component%20Object%20Reference) (OtherBodyIndex :type Integer))
  (bind _aslucero_character_bp (Utilities|Casting|CastToLuceroCharacter_BP OtherActor))
  (CallFunction|InterruptRecolect)
  (Default|RemoveCrystalRefActionable _aslucero_character_bp self))

(event OnComponentBeginOverlap(TouchCollision)
  (params (OverlappedComponent :type Primitive%20Component%20Object%20Reference) (OtherActor :type Actor%20Object%20Reference) (OtherComp :type Primitive%20Component%20Object%20Reference) (OtherBodyIndex :type Integer) (bFromSweep :type Boolean) (SweepResult :type Hit%20Result%20Structure%20%28by%20ref%29))
  (bind _aslucero_character_bp (Utilities|Casting|CastToLuceroCharacter_BP OtherActor))
  (Development|PrintString "tocando cristal")
  (Default|AddCrystalRefActionable _aslucero_character_bp self)
  (if (Variables|/Game/MyAssets/Blueprints/Character/LuceroCharacter_BP.LuceroCharacter_BP_C|GetisAuraActive? _aslucero_character_bp)
    (Utilities|FlowControl|DoOnce false
      (:Completed
        (CallFunction|ActivatePower "NewEnumerator2" 1)))))

(event OnComponentBeginOverlap(ActionCollision)
  (params (OverlappedComponent :type Primitive%20Component%20Object%20Reference) (OtherActor :type Actor%20Object%20Reference) (OtherComp :type Primitive%20Component%20Object%20Reference) (OtherBodyIndex :type Integer) (bFromSweep :type Boolean) (SweepResult :type Hit%20Result%20Structure%20%28by%20ref%29))
  (if (Variables|Default|GetisActivatedPower?)
    (bind _asenemy_pompon_bp (Utilities|Casting|CastToEnemy_Pompon_BP OtherActor))
    (CallFunction|EvaluateCollisionandAplyReaction _asenemy_pompon_bp)))

(event Custom|ControlTimerPower
  (params (DeltaTime :type Float%20%28single-precision%29))
  ;[0.9946 1 0] Timer POWER
  (if (Variables|Default|GetisActivatedPower?)
    (if (Variables|Default|GetisRecolecting?)
      (if (> (Variables|Default|GettimerPower) 0.0)
        (Variables|Default|SettimerPower (- (Variables|Default|GettimerPower) (* DeltaTime (Variables|Default|GetrecolectPotentiation))))
        (Utilities|FlowControl|DoOnce false :!label _label
          (:Completed
            (goto _label_2 Reset)))
        (else
          (Utilities|FlowControl|DoOnce false :!label _label_2
            (:Completed
              (CallFunction|DeactivatePower)
              (goto _label Reset)))))
      (elif (> (Variables|Default|GettimerPower) 0.0)
        (Variables|Default|SettimerPower (- (Variables|Default|GettimerPower) DeltaTime))
        (Utilities|FlowControl|DoOnce false :!label _label_3
          (:Completed
            (goto _label_4 Reset)))
        (else
          (Utilities|FlowControl|DoOnce false :!label _label_4
            (:Completed
              (CallFunction|DeactivatePower)
              (goto _label_3 Reset))))))))

(event Custom|ControlTimerRecolecting
  (params (DeltaTime :type Float%20%28single-precision%29))
  ;[0.9946 1 0] Timer Recolecting
  (if (and (Variables|Default|GetisRecolecting?) (<= (Variables|Default|GettimerPower) 0.0))
    (Utilities|FlowControl|DoOnce false :!label _label
      (:Completed
        (CallFunction|UnpurifyAffected)
        (Default|AddCrystal (.AsLucero%20Character%20BP (Utilities|Casting|CastToLuceroCharacter_BP (Game|GetPlayerCharacter 0))))
        (Audio|PlaySound2D "/Game/MyAssets/Sounds/UI/click_button.click_button" 1.0 1.0 0.0 0 0)
        (Actor|DestroyActor)))
    (else
      (goto _label Reset))))

(event EventBeginPlay
  (bind _output_get (Variables|Default|SetLoading_WBP_ref (.AsLoading%20WBP (Utilities|Casting|CastToloading_WBP (UserInterface|GetWidget (Variables|Default|Getloading_WBP))))))
  (Variables|/Game/MyAssets/UI/loading_WBP.loading_WBP_C|Setcrystal_ref _output_get self)
  (bind _output_get_2 (Variables|Default|SetDeactivating_WBP_ref (.AsDeactivating%20WBP (Utilities|Casting|CastTodeactivating_WBP (UserInterface|GetWidget (Variables|Default|Getdeactivating_WBP))))))
  (Variables|/Game/MyAssets/UI/deactivating_WBP.deactivating_WBP_C|Setcrystal_ref _output_get_2 self)
  (bind _output_get_3 (Variables|Default|Setcaninteract_WBP_ref (.AsCaninteract%20WBP (Utilities|Casting|CastTocaninteract_WBP (UserInterface|GetWidget (Variables|Default|Getcaninteract_WBP))))))
  (Variables|/Game/MyAssets/UI/caninteract_WBP.caninteract_WBP_C|Setcrystal_ref _output_get_3 self))

(event EventTick
  (params (DeltaSeconds :type Float%20%28single-precision%29))
  ;[1 0 0] TICK
  (Utilities|FlowControl|Sequence
    (:then_0
      (CallFunction|ControlTimerPower DeltaSeconds))
    (:then_1
      (CallFunction|ControlTimerRecolecting DeltaSeconds))))

(fn ConstructionScript
  (if (Variables|Default|GetisActivatedPower?)
    (switch Utilities|FlowControl|Switch|SwitchonPowerEnum (Variables|Default|GetPower)
      (:NewEnumerator0
        (CallFunction|ActivatePower "NewEnumerator0" 100))
      (:NewEnumerator1
        (CallFunction|ActivatePower "NewEnumerator1" 100)))))

(fn ActivatePower
  (params (Power :type PowerEnum%20Enum :default "NewEnumerator3") (SkillPoints :type Integer))
  (bind _timepotentiatorskills (Variables|Default|GetTimePotentiatorSkills))
  (bind _particlepower (Variables|Default|GetParticlePower))
  (bind _returnvalue (* SkillPoints _timepotentiatorskills))
  (bind _output_get (Variables|Default|SetPower Power))
  (Development|PrintString (Utilities|String|EnumtoString _output_get))
  (CallFunction|ChangeMaterialInstance)
  (Variables|Default|SetlastActivationMaxTime _returnvalue)
  (Variables|Default|SettimerPower _returnvalue)
  (switch Utilities|FlowControl|Switch|SwitchonPowerEnum (Variables|Default|GetPower)
    (:NewEnumerator3
      (Variables|Default|SetisActivatedPower? false)
      (Components|Activation|SetActive _particlepower false false))
    (:NewEnumerator0
      (Variables|Default|SetisActivatedPower? true)
      (Audio|PlaySound2D "/Game/MyAssets/Sounds/Actions/magic_effect2.magic_effect2" 1.0 1.0 0.0 0 0)
      (Effects|Components|ParticleSystem|SetTemplate _particlepower "/Game/StarterContent/Particles/P_Fire.P_Fire")
      (Components|Activation|SetActive _particlepower true false :!label _label)
      (Development|PrintString "Se activo el poder")
      (for _array_element (Collision|GetOverlappingActors (Variables|Default|GetActionCollision) "/Game/MyAssets/Blueprints/Enemies/Enemy_Pompon_BP.Enemy_Pompon_BP_C" :!class /Script/Engine.PrimitiveComponent)
        (bind _asenemy_pompon_bp (Utilities|Casting|CastToEnemy_Pompon_BP _array_element))
        (if (< (- (Math|Vector|VectorLength (- (Transformation|GetWorldLocation (Variables|/Script/Engine.Character|GetCapsuleComponent _asenemy_pompon_bp)) (Transformation|GetActorLocation))) 3e+01) (Variables|/Script/Engine.SphereComponent|GetSphereRadius (Variables|Default|GetActionCollision)))
          (CallFunction|EvaluateCollisionandAplyReaction _asenemy_pompon_bp))))
    (:NewEnumerator1
      (Variables|Default|SetisActivatedPower? true)
      (Audio|PlaySound2D "/Game/MyAssets/Sounds/Actions/magic_effect2.magic_effect2" 1.0 1.0 0.0 0 0)
      (Effects|Components|ParticleSystem|SetTemplate _particlepower "/Game/StarterContent/Particles/P_Smoke.P_Smoke")
      (goto _label))
    (:NewEnumerator2
      (Variables|Default|SetisActivatedPower? true)
      (Audio|PlaySound2D "/Game/MyAssets/Sounds/Actions/magic_effect2.magic_effect2" 1.0 1.0 0.0 0 0)
      (Effects|Components|ParticleSystem|SetTemplate _particlepower "/Game/StarterContent/Particles/P_Sparks.P_Sparks")
      (goto _label))))

(fn DeactivatePower
  (Components|Activation|SetActive (Variables|Default|GetParticlePower) false false)
  (Variables|Default|SettimerPower 0.0)
  (Variables|Default|SetisActivatedPower? false)
  (Variables|Default|SetPower "NewEnumerator3")
  (CallFunction|ChangeMaterialInstance)
  (CallFunction|UnpurifyAffected))

(fn RecolectCristal
  (bind _returnvalue (Game|GetPlayerCharacter 0))
  (bind _aslucero_character_bp (Utilities|Casting|CastToLuceroCharacter_BP _returnvalue))
  (if (Variables|Default|GetisActivatedPower?)
    (Variables|Default|SetisRecolecting? true)
    (else
      (Variables|/Game/MyAssets/Blueprints/Character/LuceroCharacter_BP.LuceroCharacter_BP_C|SetCrystals _aslucero_character_bp (+ (Variables|/Game/MyAssets/Blueprints/Character/LuceroCharacter_BP.LuceroCharacter_BP_C|GetCrystals _aslucero_character_bp) 1))
      (CallFunction|UnpurifyAffected)
      (Audio|PlaySound2D "/Game/MyAssets/Sounds/UI/click_button.click_button" 1.0 1.0 0.0 0 0)
      (Actor|DestroyActor))))

(fn InterruptRecolect
  (if (Variables|Default|GetisRecolecting?)
    (Variables|Default|SetisRecolecting? false)))

(fn ChangeMaterialInstance
  (bind _cube (Variables|Default|GetCube))
  (bind _pointlight (Variables|Default|GetPointLight))
  (bind _returnvalue (Rendering|Material|GetMaterials _cube))
  (switch Utilities|FlowControl|Switch|SwitchonPowerEnum (Variables|Default|GetPower)
    (:NewEnumerator3
      (for (_ _array_index) _returnvalue
        (Rendering|Material|SetMaterial _cube _array_index "/Game/MyAssets/Blueprints/Materials/Glass_MAT_inst_Black.Glass_MAT_inst_Black")
        (Rendering|SetVisibility _pointlight false false)))
    (:NewEnumerator0
      (for (_ _array_index_2) _returnvalue
        (Rendering|Material|SetMaterial _cube _array_index_2 "/Game/MyAssets/Blueprints/Materials/Glass_MAT_Inst_Yellow.Glass_MAT_Inst_Yellow")
        (Rendering|Components|Light|SetLightColor _pointlight "(R=1.000000,G=0.981161,B=0.000000,A=1.000000)" true)
        (Rendering|SetVisibility _pointlight true false)))
    (:NewEnumerator1
      (for (_ _array_index_3) _returnvalue
        (Rendering|Material|SetMaterial _cube _array_index_3 "/Game/MyAssets/Blueprints/Materials/Glass_MAT_Inst_Blue.Glass_MAT_Inst_Blue")
        (Rendering|Components|Light|SetLightColor _pointlight "(R=0.000000,G=0.140054,B=1.000000,A=1.000000)" true)
        (Rendering|SetVisibility _pointlight true false)))
    (:NewEnumerator2
      (for (_ _array_index_4) _returnvalue
        (Rendering|Material|SetMaterial _cube _array_index_4 "/Game/MyAssets/Blueprints/Materials/Glass_MAT_Inst_Red.Glass_MAT_Inst_Red")
        (Rendering|Components|Light|SetLightColor _pointlight "(R=1.000000,G=0.058563,B=0.000000,A=1.000000)" true)
        (Rendering|SetVisibility _pointlight true false)))))

(fn UnpurifyAffected
  (for _array_element (Variables|Default|GetAffectedEnemies)
    (Default|UnPurify _array_element)
    (Utilities|Array|Clear (Variables|Default|GetAffectedEnemies))))

(fn EvaluateCollisionandAplyReaction
  (params (Enemy_ref :type Enemy%20Pompon%20BP%20Object%20Reference))
  (bind _power (Variables|Default|GetPower))
  (Development|PrintString "EVALUANDO")
  (switch Utilities|FlowControl|Switch|SwitchonEnemyType (Variables|/Game/MyAssets/Blueprints/Enemies/Enemy_Pompon_BP.Enemy_Pompon_BP_C|GetEnemyType Enemy_ref)
    (:NewEnumerator0
      (switch Utilities|FlowControl|Switch|SwitchonPowerEnum _power
        (:NewEnumerator0
          _)
        (:NewEnumerator1
          _)
        (:NewEnumerator2
          _))
      (Development|PrintString "Hello" true true "(R=0.238196,G=1.000000,B=0.021221,A=1.000000)" 5.0)
      (Default|Purify Enemy_ref)
      (Utilities|Array|AddUnique (Variables|Default|GetAffectedEnemies) Enemy_ref))
    (:NewEnumerator1
      (switch Utilities|FlowControl|Switch|SwitchonPowerEnum _power
        (:NewEnumerator0
          (Default|Purify Enemy_ref :!label _label)
          (Utilities|Array|AddUnique (Variables|Default|GetAffectedEnemies) Enemy_ref))
        (:NewEnumerator1
          (goto _label))
        (:NewEnumerator2
          (Default|SetAltered Enemy_ref))))
    (:NewEnumerator2
      (switch Utilities|FlowControl|Switch|SwitchonPowerEnum _power
        (:NewEnumerator0
          (Default|SetAltered Enemy_ref :!label _label_2))
        (:NewEnumerator1
          (goto _label_2))
        (:NewEnumerator2
          (Default|Purify Enemy_ref)
          (Utilities|Array|AddUnique (Variables|Default|GetAffectedEnemies) Enemy_ref))))
    (:NewEnumerator3
      (switch Utilities|FlowControl|Switch|SwitchonPowerEnum _power
        (:NewEnumerator0
          _)
        (:NewEnumerator1
          _)
        (:NewEnumerator2
          _))
      (Default|SetSlowed Enemy_ref)
      (Development|PrintString "ENTRE AL SLOW"))))