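; Player controller for Lucero that creates the HUD, caches the game state and handles crystal actions.
; Drop and interact inputs act only while the character is alive, using DoOnce gates to limit repeat triggering.
; Interact searches the character capsule's overlaps for a Collectable-tagged crystal and starts its collection, with release feeding the interrupt/reset path.
; Number keys 1–4 push enemy state changes to the game state's level data.
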(event EventBeginPlay
  ;[1 0.1073 0.02767] Begin Play - Variables settings
  (bind _returnvalue (UserInterface|CreateWidget "/Game/MyAssets/UI/HUD_BP.HUD_BP_C"))
  (bind _output_get (Variables|Default|SetHudWidget_Ref _returnvalue))
  (UserInterface|Viewport|AddtoViewport _output_get 0)
  (bind _aslucero_gs (Utilities|Casting|CastToLucero_GS (Game|GetGameState)))
  (Variables|Default|SetLucero%20GS_Ref _aslucero_gs))

(event Input|ActionEvents|InputActionInteractWith
  (params (Key :type Key%20Structure :default "None"))
  ;[1 0.6141 0.1073] Interact with Object
  (:Pressed
    (Development|PrintString "Interact")
    (bind _isdead_ (CallFunction|CheckIsDead))
    (if (not _isdead_)
      (bind (_overlappingactionable_ _actor) (CallFunction|IsOverlappingInteractuableObject))
      (if _overlappingactionable_
        (Utilities|FlowControl|DoOnce false :!label _label
          (:Completed
            (bind _output_get (Variables|Default|SetinteractingWith_Ref _actor))
            (bind _ascrystal_bp (Utilities|Casting|CastToCrystal_BP _output_get))
            (Default|RecolectCristal _ascrystal_bp)
            (goto _label_2 Reset))))))
  (:Released
    (bind _isdead__2 (CallFunction|CheckIsDead))
    (if (not _isdead__2)
      (Utilities|FlowControl|DoOnce false :!label _label_2
        (:Completed
          (bind _output_get_2 (Variables|Default|SetinteractingWith_Ref 0))
          (Utilities|IsValid _output_get_2
            (:Is%20Valid
              (bind _ascrystal_bp_2 (Utilities|Casting|CastToCrystal_BP _output_get_2)
                (:then
                  (Default|InterruptRecolect _ascrystal_bp_2)
                  (goto _label Reset))
                (:CastFailed
                  (goto _label Reset))))
            (:Is%20Not%20Valid
              (goto _label Reset))))))))

(event Input|ActionEvents|InputActionDropCrystal
  (params (Key :type Key%20Structure :default "None"))
  (bind _returnvalue (Game|GetPlayerCharacter 0))
  (bind _returnvalue_2 (Game|GetPlayerCharacter 0))
  (bind _aslucero_character_bp (Utilities|Casting|CastToLuceroCharacter_BP _returnvalue))
  (bind _aslucero_character_bp_2 (Utilities|Casting|CastToLuceroCharacter_BP _returnvalue_2))
  ;[1 0.4876 0.1284] Drop Crystal Action
  (:Pressed
    (Development|PrintString "Drop Cristal")
    (Utilities|IsValid _aslucero_character_bp_2
      (:Is%20Valid
        (bind _isdead_ (CallFunction|CheckIsDead))
        (if (not _isdead_)
          (Utilities|FlowControl|DoOnce false :!label _label
            (:Completed
              (if (> (Variables|/Game/MyAssets/Blueprints/Character/LuceroCharacter_BP.LuceroCharacter_BP_C|GetCrystals _aslucero_character_bp) 0)
                (Default|DropCrystal _aslucero_character_bp))))))))
  (:Released
    (Utilities|IsValid _aslucero_character_bp_2
      (:Is%20Valid
        (bind _isdead__2 (CallFunction|CheckIsDead))
        (if (not _isdead__2)
          (goto _label Reset))))))

(event Input|KeyboardEvents|1
  (params (Key :type Key%20Structure :default "None"))
  (:Pressed
    (Utilities|FlowControl|DoOnce false :!label _label
      (:Completed
        (Default|UpdateCurrentLevelData (Variables|Default|GetLucero%20GS_Ref) "NewEnumerator1" false))))
  (:Released
    (goto _label Reset)))

(event Input|KeyboardEvents|2
  (params (Key :type Key%20Structure :default "None"))
  (:Pressed
    (Utilities|FlowControl|DoOnce false :!label _label
      (:Completed
        (Default|UpdateCurrentLevelData (Variables|Default|GetLucero%20GS_Ref) "NewEnumerator0" false))))
  (:Released
    (goto _label Reset)))

(event Input|KeyboardEvents|3
  (params (Key :type Key%20Structure :default "None"))
  (:Pressed
    (Utilities|FlowControl|DoOnce false :!label _label
      (:Completed
        (Default|UpdateCurrentLevelData (Variables|Default|GetLucero%20GS_Ref) "NewEnumerator2" true))))
  (:Released
    (goto _label Reset)))

(event Input|KeyboardEvents|4
  (params (Key :type Key%20Structure :default "None"))
  (:Pressed
    (Utilities|FlowControl|DoOnce false :!label _label
      (:Completed
        (Default|UpdateCurrentLevelData (Variables|Default|GetLucero%20GS_Ref) "NewEnumerator2" false))))
  (:Released
    (goto _label Reset)))

(fn ConstructionScript)

(fn IsOverlappingInteractuableObject
  (bind _returnvalue (Game|GetPlayerCharacter 0))
  (bind _aslucero_character_bp (Utilities|Casting|CastToLuceroCharacter_BP _returnvalue))
  (bind _capsulecomponent (Variables|/Script/Engine.Character|GetCapsuleComponent _aslucero_character_bp))
  (bind _overlappingactors (Collision|GetOverlappingActors _capsulecomponent 0 :!class /Script/Engine.PrimitiveComponent))
  (bind _returnvalue_2 (Utilities|Array|Length _overlappingactors))
  (Development|PrintString "Check Overlapping")
  (Development|PrintString (Utilities|String|ToString(Integer) _returnvalue_2))
  (if (> _returnvalue_2 0)
    (for _array_element _overlappingactors
      (if (Actor|ActorHasTag _array_element "Collectable")
        (bind _ascrystal_bp (Utilities|Casting|CastToCrystal_BP _array_element))
        (return (Actor|ActorHasTag _array_element "Collectable") _ascrystal_bp)))
    (else
      (Development|PrintString "No overlapping")))
  (return false 0))

(fn CheckIsDead
  (bind _returnvalue (Game|GetPlayerCharacter 0))
  (bind _aslucero_character_bp (Utilities|Casting|CastToLuceroCharacter_BP _returnvalue))
  (Utilities|IsValid _aslucero_character_bp
    (:Is%20Valid
      (return (Variables|/Game/MyAssets/Blueprints/Character/LuceroCharacter_BP.LuceroCharacter_BP_C|GetisDead? _aslucero_character_bp)))
    (:Is%20Not%20Valid
      (return true))))