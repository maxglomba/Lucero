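; Game state Blueprint that tracks each level's light and dark creature counts and uses them to control that level's doors.
; InitLevel selects the current level and starts all its creatures as dark.
; UpdateCurrentLevelData applies To Dark, To Light or Kill changes, guarding against negative counts; killed totals are derived from the remainder.
; After each applied change, CheckDoorState opens every door in DoorsLevel when lighted creatures equal or outnumber dark ones, otherwise closes them.
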(event EventBeginPlay)

(event EventTick
  (params (DeltaSeconds :type Float%20%28single-precision%29)))

(fn ConstructionScript)

(fn InitLevel
  (params (Base%20Creatures :type Integer) (Level :type Integer))
  (bind _returnvalue (- Level 1))
  (bind _leveldata (Variables|Default|GetLevelData))
  (bind _output (Utilities|Array|Get(acopy) _leveldata _returnvalue))
  (bind (_id _name) (Utilities|Struct|BreakLevelStructure _output))
  (Variables|Default|SetcurrentLevel Level)
  (Utilities|Array|SetArrayElem _leveldata _returnvalue (Utilities|Struct|MakeLevelStructure _id _name Base%20Creatures 0 Base%20Creatures))
  (CallFunction|CheckDoorState))

(fn GetCurrentLevelData
  (bind _currentlevel (Variables|Default|GetcurrentLevel))
  (bind _leveldata (Variables|Default|GetLevelData))
  (bind _returnvalue (- _currentlevel 1))
  (bind _output (Utilities|Array|Get(acopy) _leveldata _returnvalue))
  (bind (_id _name _basecreatures _lighted _darked) (Utilities|Struct|BreakLevelStructure _output))
  (return _name _basecreatures _lighted _darked (- (- _basecreatures _lighted) _darked) _id (>= _lighted _darked)))

(fn UpdateCurrentLevelData
  (params (AffectEnemyState :type AffectEnemyState%20Enum :default "NewEnumerator0") (isDarkEnemy? :type Boolean))
  (bind _leveldata (Variables|Default|GetLevelData))
  (bind _currentlevel (Variables|Default|GetcurrentLevel))
  (bind _returnvalue (- _currentlevel 1))
  (bind _output_get (Variables|Default|SetAffectEnemyState AffectEnemyState))
  (bind (_name _base_creatures _lighted _darked _killed _id) (CallFunction|GetCurrentLevelData))
  (switch Utilities|FlowControl|Switch|SwitchonAffectEnemyState _output_get
    (:NewEnumerator0
      (if (>= (- _lighted 1) 0)
        (Utilities|Array|SetArrayElem _leveldata _returnvalue (Utilities|Struct|MakeLevelStructure _id _name _base_creatures (- _lighted 1) (+ _darked 1)))
        (CallFunction|CheckDoorState :!label _label)))
    (:NewEnumerator1
      (if (>= (- _darked 1) 0)
        (Utilities|Array|SetArrayElem _leveldata _returnvalue (Utilities|Struct|MakeLevelStructure _id _name _base_creatures (+ _lighted 1) (- _darked 1)))
        (goto _label)))
    (:NewEnumerator2
      (if isDarkEnemy?
        (if (>= (- _darked 1) 0)
          (Utilities|Array|SetArrayElem _leveldata _returnvalue (Utilities|Struct|MakeLevelStructure _id _name _base_creatures _lighted (- _darked 1)))
          (goto _label))
        (elif (>= (- _lighted 1) 0)
          (Utilities|Array|SetArrayElem _leveldata _returnvalue (Utilities|Struct|MakeLevelStructure _id _name _base_creatures (- _lighted 1) _darked))
          (goto _label))))))

(fn CheckDoorState
  (bind _doorslevel (Variables|Default|GetDoorsLevel))
  (bind _openeddoor (CallFunction|GetCurrentLevelData))
  (if _openeddoor
    (for _array_element _doorslevel
      (Default|ChangeStateDoor _array_element true))
    (else
      (for _array_element_2 _doorslevel
        (Default|ChangeStateDoor _array_element_2 false)))))