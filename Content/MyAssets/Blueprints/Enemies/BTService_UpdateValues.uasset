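; Behavior tree service that mirrors the Pompon enemy's state into its blackboard on each AI tick.
; It casts the controlled pawn to Enemy_Pompon_BP and copies its last known player location, player reference, attacking state and purified flag into blackboard keys.
; The CanSeePlayer key is set when true and cleared otherwise, while the InAttackZone key is fed from the pawn's IsAttacking flag.
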(event EventReceiveTickAI
  (params (OwnerController :type AI%20Controller%20Object%20Reference) (ControlledPawn :type Pawn%20Object%20Reference) (DeltaSeconds :type Float%20%28single-precision%29))
  (bind _canseeplayerkey (Variables|Default|GetcanSeePlayerKey))
  (bind _asenemy_pompon_bp (Utilities|Casting|CastToEnemy_Pompon_BP ControlledPawn))
  (if (Variables|/Game/MyAssets/Blueprints/Enemies/Enemy_Pompon_BP.Enemy_Pompon_BP_C|GetcanSeePlayer _asenemy_pompon_bp)
    (Class|BTFunctionLibrary|SetBlackboardValueasBool _canseeplayerkey true)
    (else
      (Class|BTFunctionLibrary|ClearBlackboardValue _canseeplayerkey)))
  (AI|BehaviorTree|SetBlackboardValueasVector (Variables|Default|GetlastKnowPlayerLocationKey) (Variables|/Game/MyAssets/Blueprints/Enemies/Enemy_Pompon_BP.Enemy_Pompon_BP_C|GetlastPlayerLocation _asenemy_pompon_bp))
  (Class|BTFunctionLibrary|SetBlackboardValueasObject (Variables|Default|GetplayerRefKey) (Variables|/Game/MyAssets/Blueprints/Enemies/Enemy_Pompon_BP.Enemy_Pompon_BP_C|GetplayerRef _asenemy_pompon_bp))
  (Class|BTFunctionLibrary|SetBlackboardValueasBool (Variables|Default|GetinAttackZone) (Variables|/Game/MyAssets/Blueprints/Enemies/Enemy_Pompon_BP.Enemy_Pompon_BP_C|GetisAttacking? _asenemy_pompon_bp))
  (Class|BTFunctionLibrary|SetBlackboardValueasBool (Variables|Default|GetpurifiedKey) (Variables|/Game/MyAssets/Blueprints/Enemies/Enemy_Pompon_BP.Enemy_Pompon_BP_C|Getpurified _asenemy_pompon_bp)))