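; Behavior tree task that picks a random location for the Pompon enemy around the player's last known location.
; It writes a vector to the random location blackboard key, taking Y and Z from a random navigable point within the radius and X from the enemy's own position.
; It then finishes successfully, but a failed cast to Enemy_Pompon_BP stops it without finishing.
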(event EventReceiveExecuteAI
  (params (OwnerController :type AI%20Controller%20Object%20Reference) (ControlledPawn :type Pawn%20Object%20Reference))
  (bind _radius (Variables|Default|GetRadius))
  (bind _lastknowplayerlocation (Variables|Default|GetlastKnowPlayerLocation))
  (bind _returnvalue (Class|BTFunctionLibrary|GetBlackboardValueasVector _lastknowplayerlocation))
  (bind _randomlocation (Class|NavigationSystemV1|GetRandomPointinNavigableRadius _returnvalue _radius 0 0))
  (bind _asenemy_pompon_bp (Utilities|Casting|CastToEnemy_Pompon_BP (Class|BTFunctionLibrary|GetBlackboardValueasObject (Variables|Default|GetobjectRefKey))))
  (AI|BehaviorTree|SetBlackboardValueasVector (Variables|Default|GetrandomlocationKey) (Math|Vector|MakeVector (.x (Transformation|GetActorLocation _asenemy_pompon_bp)) (.y _randomlocation) (.z _randomlocation)))
  (AI|BehaviorTree|FinishExecute true))